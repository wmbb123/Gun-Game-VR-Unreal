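; VR game mode Blueprint that runs timed waves of enemy spawns once StartGame is called.
; BeginPlay caches every actor implementing BPI_EnemySpawner.
; Each wave shuffles those spawners and messages as many as EnemiesPerWave lists for it, so each picked spawner is distinct.
; SpawnEnemyWave then re-arms itself by timer after DelayPW until the wave list runs out.
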(event `self.ReceiveBeginPlay`
  (bind _outactors (`GameplayStatics.GetAllActorsWithInterface` "/Game/Blueprints/Enemy/BPI_EnemySpawner.BPI_EnemySpawner_C"))
  (set `self.EnemySpawners` _outactors))

(event `/Game/Blueprints/Gamemode/BPI_Gamemode.StartGame`
  (`self.SpawnEnemyWave`))

(fn `SpawnEnemyWave`
  (if (not (> (`self.CurrentWNumber`) (`KismetArrayLibrary.Array_LastIndex` (`self.EnemiesPerWave`))))
    (`KismetArrayLibrary.Array_Shuffle` (`self.EnemySpawners`))
    (for _index (range (`|GetArrayItem` (`self.EnemiesPerWave`) (`self.CurrentWNumber`)))
      (message `/Game/Blueprints/Enemy/BPI_EnemySpawner.HandleEnemySpanwer` (`|GetArrayItem` (`self.EnemySpawners`) _index)))
    (`/Engine/EditorBlueprintResources/StandardMacros.IncrementInt` (`self.CurrentWNumber`)
      (:`  `
        (`KismetSystemLibrary.K2_SetTimer` null "SpawnEnemyWave" (`self.DelayPW`))))))

(fn `UserConstructionScript`)