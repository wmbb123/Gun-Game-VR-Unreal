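; Player Blueprint that handles shooting and score keeping, with firing bound to an Oculus right input.
; Each press line traces forward from FiringStart, spawns smoke at the impact and messages the hit actor through the enemy or menu interface.
; It finds the in-game score display by interface on BeginPlay and pushes the total to it whenever score is added or reset.
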(event `InputAction|OculusRight`
  (params (Key :type "Key Structure"))
  (bind _firingstart (`self.FiringStart`))
  (bind _returnvalue (`SceneComponent.K2_GetComponentLocation` _firingstart))
  (:`Pressed`
    (bind (_outhit _returnvalue_2) (`KismetSystemLibrary.LineTraceSingle` _returnvalue (+ _returnvalue (* (`KismetMathLibrary.GetForwardVector` (`SceneComponent.K2_GetComponentRotation` _firingstart)) 1500.0)) "TraceTypeQuery1"))
    (if _returnvalue_2
      (bind (_bblockinghit _binitialoverlap _time _distance _location _impactpoint _normal _impactnormal _physmat _hitactor _hitcomponent) (`GameplayStatics.BreakHitResult` _outhit))
      (set `self.HitActor` _hitactor)
      (`GameplayStatics.SpawnEmitterAtLocation` "/Game/Materials/PS_Smoke.PS_Smoke" _impactpoint (`KismetMathLibrary.MakeRotFromZ` _impactnormal))
      (if (`KismetSystemLibrary.DoesImplementInterface` (`self.HitActor`) "/Game/Blueprints/Enemy/BPI_Enemy.BPI_Enemy_C")
        (message `/Game/Blueprints/Enemy/BPI_Enemy.EnemyHit` (`self.HitActor`))
        (elif (`KismetSystemLibrary.DoesImplementInterface` (`self.HitActor`) "/Game/Blueprints/Menu/BPI_Menu.BPI_Menu_C")
          (message `/Game/Blueprints/Menu/BPI_Menu.InteractiveWMenu` (`self.HitActor`) _hitcomponent))))))

(event `self.ReceiveBeginPlay`
  (bind _outactors (`GameplayStatics.GetAllActorsWithInterface` "/Game/Blueprints/UI/BPI_InGameScore.BPI_InGameScore_C"))
  (set `self.ScoreBP` (`|GetArrayItem` _outactors)))

(event `/Game/Blueprints/Player/BPI_Player.AddToScore`
  (params (Value :type Integer))
  (bind _output_get (set `self.PlayerScore` (+ (`self.PlayerScore`) Value)))
  (message `/Game/Blueprints/UI/BPI_InGameScore.UpdateDisplayedScore` (`self.ScoreBP`) _output_get))

(event `/Game/Blueprints/Player/BPI_Player.ResetScore`
  (bind _output_get (set `self.PlayerScore` 0))
  (message `/Game/Blueprints/UI/BPI_InGameScore.UpdateDisplayedScore` (`self.ScoreBP`) _output_get))

(fn `UserConstructionScript`)