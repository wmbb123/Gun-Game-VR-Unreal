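; User is a VR player Blueprint that line traces forward from its FireStart component when the Oculus right controller input is pressed.
; The trace uses the Visibility channel, but nothing follows its hit check.
; A disconnected, never-run chain would spawn smoke at the impact, then send a hit message through BPI_Enemy or pass the hit component through BPI_Menu.
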(event `InputAction|OculusRightContoller`
  (params (Key :type "Key Structure"))
  (bind _firestart (`self.FireStart`))
  (bind _returnvalue (`SceneComponent.K2_GetComponentLocation` _firestart))
  (:`Pressed`
    (bind (_outhit _returnvalue_2) (`KismetSystemLibrary.LineTraceSingle` _returnvalue (+ _returnvalue (* (`KismetMathLibrary.GetForwardVector` (`SceneComponent.K2_GetComponentRotation` _firestart)) 1500.0)) "TraceTypeQuery1"))
    (if _returnvalue_2
      _)))

(fn `UserConstructionScript`)